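; BP_P38 is a P38 aircraft actor that flies forward along its local X axis while spinning its two propellers.
; Each Tick calls MoveForward to offset the actor by MoveSpeed, scaled by world delta seconds.
; Both propellers roll at RotateSpeed with the same scaling, the left inside RotatePropeller and the right directly in the Tick graph.
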(event `self.ReceiveTick`
  (params (DeltaSeconds :type "Float (single-precision)"))
  (`self.Move Forward`)
  (`self.Rotate Propeller`)
  ;[1 1 1] Rolling Right Propeller
  (`SceneComponent.K2_AddLocalRotation` (`self.Right`) (`KismetMathLibrary.MakeRotator` (* (`GameplayStatics.GetWorldDeltaSeconds`) (`self.Rotate Speed`))) false false))

(fn `Move Forward`
  ;[1 1 1] Move Forward
  (`self.K2_AddActorLocalOffset` (`KismetMathLibrary.MakeVector` (* (`GameplayStatics.GetWorldDeltaSeconds`) (`self.Move Speed`)))))

(fn `Rotate Propeller`
  ;[1 1 1] Rolling Left Propeller
  (`SceneComponent.K2_AddLocalRotation` (`self.Left`) (`KismetMathLibrary.MakeRotator` (* (`GameplayStatics.GetWorldDeltaSeconds`) (`self.Rotate Speed`))) false false))

(fn `UserConstructionScript`)