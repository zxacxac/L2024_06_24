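; BP_P37 is a player-controlled plane that constantly moves along its forward vector while spinning its Right and Left components.
; Pitch and roll axes rotate the actor locally at a frame-rate-independent rate, and the booster input raises forward speed while held.
; Fire alternates between two arrow-mounted launch points via FlipFlop, spawning BP_Rocket.
; Each side has its own two-second cooldown, during which its rocket component is hidden.
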(event `InputAxis|PITCH`
  (params (AxisValue :type "Float (single-precision)"))
  (`self.K2_AddActorLocalRotation` (`KismetMathLibrary.MakeRotator` 0.0 (* (`KismetMathLibrary.FClamp` AxisValue -1.0 1.0) 60.0 (`GameplayStatics.GetWorldDeltaSeconds`)))))

(event `InputAxis|ROLL`
  (params (AxisValue :type "Float (single-precision)"))
  (`self.K2_AddActorLocalRotation` (`KismetMathLibrary.MakeRotator` (* (`KismetMathLibrary.FClamp` AxisValue -1.0) 60.0 (`GameplayStatics.GetWorldDeltaSeconds`)))))

(event `self.ReceiveTick`
  (params (DeltaSeconds :type "Float (single-precision)"))
  (`self.AddMovementInput` (`self.GetActorForwardVector`) (`self.Scale Value`))
  (`SceneComponent.K2_AddLocalRotation` (`self.Right`) (`KismetMathLibrary.MakeRotator` (* (`self.Rotate Speed`) (`GameplayStatics.GetWorldDeltaSeconds`))) false false)
  (`SceneComponent.K2_AddLocalRotation` (`self.Left`) (`KismetMathLibrary.MakeRotator` (* (`self.Rotate Speed`) (`GameplayStatics.GetWorldDeltaSeconds`))) false false))

(event `InputAction|BOOSTER`
  (params (Key :type "Key Structure"))
  (:`Pressed`
    (set `self.Scale Value` 1.0))
  (:`Released`
    (set `self.Scale Value` 0.5)))

(event `InputAction|FIRE`
  (params (Key :type "Key Structure"))
  (:`Pressed`
    (`/Engine/EditorBlueprintResources/StandardMacros.FlipFlop`
      (:`A`
        (if (`self.NewVar`)
          (`|SpawnActorFromClass` "/Game/P38/BP_Rocket.BP_Rocket_C" (`SceneComponent.K2_GetComponentToWorld` (`self.Arrow`)) "Undefined" "MultiplyWithRoot" null null)
          (set `self.NewVar` false)
          (`SceneComponent.SetVisibility` (`self.Left Rocket`) (`self.NewVar`) false)
          (`KismetSystemLibrary.Delay` 2.0)
          (set `self.NewVar` true)
          (`SceneComponent.SetVisibility` (`self.Left Rocket`) (`self.NewVar`) false)))
      (:`B`
        (if (`self.NewVar_0`)
          (`|SpawnActorFromClass` "/Game/P38/BP_Rocket.BP_Rocket_C" (`SceneComponent.K2_GetComponentToWorld` (`self.Arrow1`)) "Undefined" "MultiplyWithRoot" null null)
          (set `self.NewVar_0` false)
          (`SceneComponent.SetVisibility` (`self.Right Rocket`) (`self.NewVar_0`) false)
          (`KismetSystemLibrary.Delay` 2.0)
          (set `self.NewVar_0` true)
          (`SceneComponent.SetVisibility` (`self.Right Rocket`) (`self.NewVar_0`) false))))))

(fn `UserConstructionScript`)